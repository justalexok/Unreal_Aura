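; BP_EnemyBase is the base enemy character Blueprint, handling spawn, facing and dissolve visuals.
; On BeginPlay a timeline animates the mesh's uniform scale.
; SetFacingTarget updates a Motion Warping target named FacingTarget with a given location.
; Two dissolve events, one general and one for the weapon, run separate timelines that drive the Dissolve scalar on a supplied dynamic material instance.
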(event EventBeginPlay
  (bind _scaletrack (Timeline|Spawn%20Timeline Play)
    (:Update
      (Transformation|SetRelativeScale3D (Variables|Character|GetMesh) (Math|Vector|MakeVector _scaletrack _scaletrack _scaletrack)))))

(event Collision|EventActorBeginOverlap
  (params (OtherActor :type Actor%20Object%20Reference)))

(event EventTick
  (params (DeltaSeconds :type Float%20%28single-precision%29)))

(event EventStartDissolveTimeline
  (params (DynamicMaterialInstance :type Material%20Instance%20Dynamic%20Object%20Reference))
  (bind _dissolve_track (Timeline|Dissolve%20TImeline Play)
    (:Update
      (Rendering|Material|SetScalarParameterValue DynamicMaterialInstance "Dissolve" _dissolve_track :!class /Script/Engine.MaterialInstanceDynamic))))

(event EventStartWeaponDissolveTimeline
  (params (DynamicMaterialInstance :type Material%20Instance%20Dynamic%20Object%20Reference))
  (bind _weapon_dissolve_track (Timeline|Weapon%20Dissolve%20Timeline Play)
    (:Update
      (Rendering|Material|SetScalarParameterValue DynamicMaterialInstance "Dissolve" _weapon_dissolve_track :!class /Script/Engine.MaterialInstanceDynamic))))

(event EventSetFacingTarget
  (params (FacingTarget :type Vector%20%28by%20ref%29 :default "0, 0, 0"))
  (Class|MotionWarpingComponent|AddorUpdateWarpTargetfromLocation (Variables|Default|GetMotionWarping) "FacingTarget" FacingTarget))

(fn ConstructionScript)