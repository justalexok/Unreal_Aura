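; Melee attack gameplay ability for enemies, damaging hostile live players near the striking point.
; It turns the avatar toward its combat target, then plays a random tagged montage from the avatar's attack montages.
; When the montage's gameplay event arrives, it runs a small sphere query at that tag's combat socket and damages non-friends.
; The ability ends after that hit check, or when the montage completes, is interrupted or is cancelled.
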(event Ability|EventActivateAbility
  (bind _returnvalue (Ability|GetAvatarActorfromActorInfo))
  (bind _returnvalue_2 (Ability|GetAvatarActorfromActorInfo))
  ;[0.06393 0.004579 0.0816] Face Target
  (bind _returnvalue_3 (Class|EnemyInterface|GetCombatTarget(Message) _returnvalue_2))
  (Class|CombatInterface|SetFacingTarget(Message) _returnvalue_2 (Transformation|GetActorLocation _returnvalue_3))
  ;[0.00302 0.07465 0.03917] Montage
  (bind _returnvalue_4 (Class|CombatInterface|GetAttackMontages(Message) (Ability|GetAvatarActorfromActorInfo)))
  (bind _returnvalue_5 (Class|AuraDamageGameplayAbility|GetRandomTaggedMontage _returnvalue_4))
  (bind _output_get (Variables|Default|SetTagged%20Montage _returnvalue_5))
  (|PlayMontageandWaitProxy "None" (.AnimMontage (Utilities|Struct|BreakTaggedMontage _output_get)) 1.0 "None" false 1.0 0.0 false
    (:then
      (Ability|Tasks|WaitGameplayEvent (.MontageTag (Utilities|Struct|BreakTaggedMontage _output_get)) 0
        (:EventReceived
          ;[0.005835 0.06814 0.2066] Cause Damage to nearby foes
          (bind _returnvalue_6 (Class|CombatInterface|GetCombatSocketLocation(Message) _returnvalue (.MontageTag (Utilities|Struct|BreakTaggedMontage _output_get))))
          (bind _outoverlappingactors (Class|AuraAbilitySystemLibrary|GetLivePlayersWithinRadius _returnvalue (Utilities|Array|MakeArray _returnvalue) 45.0 _returnvalue_6))
          (for _array_element _outoverlappingactors
            (if (Class|AuraAbilitySystemLibrary|IsNotFriend (Ability|GetAvatarActorfromActorInfo) _array_element)
              (Class|AuraDamageGameplayAbility|CauseDamage _array_element)))
          (Ability|EndAbility))))
    (:OnCompleted
      (Ability|EndAbility :!label _label))
    (:OnInterrupted
      (goto _label))
    (:OnCancelled
      (goto _label))))

(event Ability|EventOnEndAbility
  (params (bWasCancelled :type Boolean)))