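; GA_RangedAttack is an enemy gameplay ability that fires a projectile at the avatar's combat target.
; On activation it turns the avatar toward the target and plays a random tagged attack montage.
; A one-shot wait for that montage's gameplay event tag then spawns the projectile from its socket tag toward the target's current location, with optional pitch override, and ends the ability.
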(event Ability|EventActivateAbility
  (bind _returnvalue (Ability|GetAvatarActorfromActorInfo))
  ;[0.06393 0.004579 0.0816] Face Target
  (bind _returnvalue_2 (Class|EnemyInterface|GetCombatTarget(Message) _returnvalue))
  (Class|CombatInterface|SetFacingTarget(Message) _returnvalue (Transformation|GetActorLocation _returnvalue_2))
  ;[0.00302 0.07465 0.03917] Montage
  (bind _returnvalue_3 (Class|CombatInterface|GetAttackMontages(Message) (Ability|GetAvatarActorfromActorInfo)))
  (Variables|Default|SetTaggedMontage (Class|AuraDamageGameplayAbility|GetRandomTaggedMontage _returnvalue_3))
  (|PlayMontageandWaitProxy "None" (.animmontage (Variables|Default|GetTaggedMontage)) 1.0 "None" false 1.0 0.0 false
    (:then
      (Ability|Tasks|WaitGameplayEvent (.montagetag (Variables|Default|GetTaggedMontage)) 0 true
        (:EventReceived
          (bind _returnvalue_4 (Class|EnemyInterface|GetCombatTarget(Message) (Ability|GetAvatarActorfromActorInfo)))
          (Class|AuraProjectileSpell|SpawnProjectile (Transformation|GetActorLocation _returnvalue_4) (.sockettag (Variables|Default|GetTaggedMontage)) (Variables|Default|GetShould%20Override%20Pitch) (Variables|Default|GetPitch%20Overide))
          (Ability|EndAbility))))))

(event Ability|EventOnEndAbility
  (params (bWasCancelled :type Boolean)))